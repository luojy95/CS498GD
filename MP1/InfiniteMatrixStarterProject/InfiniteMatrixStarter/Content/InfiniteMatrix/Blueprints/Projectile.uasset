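; Projectile actor that flies in a straight line and removes itself when it hits static mesh geometry.
; Tick moves it along world X by MovingSpeed scaled by delta time, setting location without sweep, regardless of the actor's rotation.
; When the Bullet component begins overlapping a StaticMeshComponent, the actor destroys itself after a short delay; it applies no damage or other effect.
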(event `self.ReceiveTick`
  (params (DeltaSeconds :type "Float (single-precision)"))
  (bind (_returnvalue_x _returnvalue_y _returnvalue_z) (`KismetMathLibrary.BreakVector` (`self.K2_GetActorLocation` self)))
  (`self.K2_SetActorLocation` (`KismetMathLibrary.MakeVector` (+ _returnvalue_x (* DeltaSeconds (`self.MovingSpeed`))) _returnvalue_y _returnvalue_z)))

(event `self.Bullet.OnComponentBeginOverlap`
  (params (OverlappedComponent :type "PrimitiveComponent Object Reference") (OtherActor :type "Actor Object Reference") (OtherComp :type "PrimitiveComponent Object Reference") (OtherBodyIndex :type Integer) (bFromSweep :type Boolean) (SweepResult :type "HitResult Structure (by ref)"))
  (cast `StaticMeshComponent` OtherComp)
  (`KismetSystemLibrary.Delay` 0.1)
  (`self.K2_DestroyActor`))

(fn `UserConstructionScript`)